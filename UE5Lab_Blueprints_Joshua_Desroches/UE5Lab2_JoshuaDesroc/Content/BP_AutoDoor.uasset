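; Automatic door Blueprint that swings its static mesh open when something overlaps its Box trigger and closes it afterwards.
; BeginPlay caches the closed rotation and derives the open one by setting yaw to OpenAngle; a timeline lerps between them.
; End overlap waits CloseDelay, then reverses the timeline only if the box is empty, clearing IsOpen on finish.
; ForceOpen and ForceClose set IsOpen and drive the timeline directly.
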(event OnComponentEndOverlap(Box)
  (params (OverlappedComponent :type Primitive%20Component%20Object%20Reference) (OtherActor :type Actor%20Object%20Reference) (OtherComp :type Primitive%20Component%20Object%20Reference) (OtherBodyIndex :type Integer))
  (Utilities|FlowControl|Delay (Variables|Default|GetCloseDelay))
  (if (Utilities|Array|IsEmpty (Collision|GetOverlappingActors (Variables|Default|GetBox) 0 :!class /Script/Engine.PrimitiveComponent))
    (Development|PrintString "Closing Door")
    (bind _alpha (Timeline|TL_Door Reverse)
      (:Update
        (Transformation|SetRelativeRotation (Variables|Default|GetStaticMesh) (Math|Rotator|Lerp(Rotator) (Variables|Default|GetClosedRot) (Variables|Default|GetOpenRot) _alpha) false false))
      (:Finished
        (Variables|Default|SetIsOpen false)))))

(event OnComponentBeginOverlap(Box)
  (params (OverlappedComponent :type Primitive%20Component%20Object%20Reference) (OtherActor :type Actor%20Object%20Reference) (OtherComp :type Primitive%20Component%20Object%20Reference) (OtherBodyIndex :type Integer) (bFromSweep :type Boolean) (SweepResult :type Hit%20Result%20Structure%20%28by%20ref%29))
  (if (not (Variables|Default|GetIsOpen))
    (Development|PrintString "Open Door")
    (Variables|Default|SetIsOpen true)
    (bind _alpha (Timeline|TL_Door Play)
      (:Update
        (Transformation|SetRelativeRotation (Variables|Default|GetStaticMesh) (Math|Rotator|Lerp(Rotator) (Variables|Default|GetClosedRot) (Variables|Default|GetOpenRot) _alpha) false false))
      (:Finished
        (Variables|Default|SetIsOpen false)))))

(event EventBeginPlay
  (bind _output_get (Variables|Default|SetClosedRot (Variables|/Script/Engine.SceneComponent|GetRelativeRotation (Variables|Default|GetStaticMesh))))
  (Variables|Default|SetOpenRot (Math|Rotator|MakeRotator (.Roll (Math|Rotator|BreakRotator _output_get)) (.Pitch (Math|Rotator|BreakRotator _output_get)) (Variables|Default|GetOpenAngle))))

(fn ConstructionScript)

(fn ForceOpen
  (Variables|Default|SetIsOpen true)
  (Audio|Components|Audio|Play (Variables|Default|GetTL_Door)))

(fn ForceClose
  (Variables|Default|SetIsOpen false)
  (Utilities|String|Reverse (Variables|Default|GetTL_Door)))